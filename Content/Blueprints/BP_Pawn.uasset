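; Player pawn for a lane-based game that switches lanes and cycles between three shapes.
; On BeginPlay it reads lane count and width from the Level Manager and sets its current lane to the middle.
; A/D or arrow keys run timelines that lerp Y to the neighbouring lane, guarded by edge checks and a Moving flag.
; Space drives a looping MultiGate that toggles visibility of the three Player components to shapeshift.
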(event `self.ReceiveBeginPlay`
  (`self.Initialise`))

(event `Key|A`
  (params (Key :type "Key Structure"))
  (bind (_returnvalue_x _returnvalue_y _returnvalue_z) (`KismetMathLibrary.BreakVector` (`self.K2_GetActorLocation`)))
  (bind (_returnvalue_x_2 _returnvalue_y_2) (`KismetMathLibrary.BreakVector` (`self.K2_GetActorLocation`)))
  ;[1 1 1] MoveLeft
  (:`Pressed`
    ;;[1 1 1] Pressed left in left most lane
    (if (<= (`self.CurrentLane`) 1) :!label _label
      _
      (elif (not (`self.bMoving`))
        (set `self.bMoving` true)
        (set `self.TargetPosition` (- _returnvalue_y_2 (`self.LaneWidth`)))
        (bind (_direction _move) (`Timeline|MoveLeft` :!via `PlayFromStart`)
          (:`Update`
            (`self.K2_SetActorLocation` (`KismetMathLibrary.MakeVector` 0.0 (`KismetMathLibrary.Lerp` _returnvalue_y (`self.TargetPosition`) _move) _returnvalue_z)))
          (:`Finished`
            (set `self.bMoving` false)
            (`/Engine/EditorBlueprintResources/StandardMacros.DecrementInt` (`self.CurrentLane`))))))))

(event `Key|Left`
  (params (Key :type "Key Structure"))
  ;[1 1 1] MoveLeft
  (:`Pressed`
    (goto _label)))

(event `Key|D`
  (params (Key :type "Key Structure"))
  (bind (_returnvalue_x _returnvalue_y) (`KismetMathLibrary.BreakVector` (`self.K2_GetActorLocation`)))
  (bind (_returnvalue_x_2 _returnvalue_y_2 _returnvalue_z) (`KismetMathLibrary.BreakVector` (`self.K2_GetActorLocation`)))
  ;[1 1 1] MoveRight
  (:`Pressed`
    ;;[1 1 1] Check if right is pressed at right most lane
    (if (== (`self.CurrentLane`) (`/Game/Blueprints/BP_LevelManager.NumberOfLanes` (`self.LevelManagerRef`))) :!label _label_2
      _
      (elif (not (`self.bMoving`))
        (set `self.bMoving` true)
        (set `self.TargetPosition` (+ _returnvalue_y (`self.LaneWidth`)))
        (bind (_direction _move) (`Timeline|MoveRight` :!via `PlayFromStart`)
          (:`Update`
            (`self.K2_SetActorLocation` (`KismetMathLibrary.MakeVector` 0.0 (`KismetMathLibrary.Lerp` _returnvalue_y_2 (`self.TargetPosition`) _move) _returnvalue_z)))
          (:`Finished`
            (set `self.bMoving` false)
            (`/Engine/EditorBlueprintResources/StandardMacros.IncrementInt` (`self.CurrentLane`))))))))

(event `Key|Right`
  (params (Key :type "Key Structure"))
  ;[1 1 1] MoveRight
  (:`Pressed`
    (goto _label_2)))

(event `Key|SpaceBar`
  (params (Key :type "Key Structure"))
  ;[1 1 1] Shapeshifting mechanics
  (:`Pressed`
    (`|MultiGate` false true
      (:`Out 0`
        (`SceneComponent.SetVisibility` (`self.Player`) false false)
        (`SceneComponent.SetVisibility` (`self.Player2`) true false))
      (:`Out 1`
        (`SceneComponent.SetVisibility` (`self.Player2`) false false)
        (`SceneComponent.SetVisibility` (`self.Player3`) true false))
      (:`Out 2`
        (`SceneComponent.SetVisibility` (`self.Player3`) false false)
        (`SceneComponent.SetVisibility` (`self.Player`) true false)))))

(fn `Initialise`
  (bind _output (`/Game/Blueprints/library/BPM_Lib.GetLevelManager`)
    (:`Is Valid`
      (set `self.LevelManagerRef` _output)
      (set `self.CurrentLane` (+ (/ (`/Game/Blueprints/BP_LevelManager.NumberOfLanes` (`self.LevelManagerRef`)) 2) 1))
      (set `self.LaneWidth` (`/Game/Blueprints/BP_LevelManager.Lanewidth` (`self.LevelManagerRef`))))
    (:`Is Not Valid`
      (`KismetSystemLibrary.PrintString` "No Level Manager Found"))))

(fn `UserConstructionScript`)